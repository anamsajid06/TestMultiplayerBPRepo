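; Networking demo actor that contrasts a multicast event with a RepNotify variable, using a cube and a trigger box.
; On overlap, the server calls a multicast that spawns a one-off explosion at the cube and sets SwitchMaterial.
; OnRep_SwitchMaterial turns the cube to rusted metal, a persistent state change unlike the transient effect.
; The construction script sets the description text and sizes a glass sphere from the net cull distance.
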(event `self.BoxCollision.OnComponentBeginOverlap`
  (params (OverlappedComponent :type "PrimitiveComponent Object Reference") (OtherActor :type "Actor Object Reference") (OtherComp :type "PrimitiveComponent Object Reference") (OtherBodyIndex :type Integer) (bFromSweep :type Boolean) (SweepResult :type "HitResult Structure (by ref)"))
  (`/Engine/EditorBlueprintResources/ActorMacros.Switch Has Authority`
    (:`Authority`
      (`self.OverlappingBox_Multicast`))))

(event `OverlappingBox_Multicast`
  (`GameplayStatics.SpawnEmitterAtLocation` "/Game/StarterContent/Particles/P_Explosion.P_Explosion" (`SceneComponent.K2_GetComponentLocation` (`self.Cube`)) (struct) (2.0 2.0 2.0))
  (set `self.SwitchMaterial` true))

(fn `OnRep_SwitchMaterial`
  (if (`self.SwitchMaterial`)
    (`PrimitiveComponent.SetMaterial` (`self.Cube`) 0 "/Game/StarterContent/Materials/M_Metal_Rust.M_Metal_Rust")))

(fn `UserConstructionScript`
  ;[1 1 1] Set glass sphere scale
  (`SceneComponent.SetWorldScale3D` (`self.GlassSphere`) (`KismetMathLibrary.Conv_DoubleToVector` (/ (`KismetMathLibrary.Sqrt` (`self.NetCullDistanceSquared`)) 50.0)))
  ;[1 1 1] Set description
  (`TextRenderComponent.K2_SetText` (`self.TextRender`) (`self.Description`)))