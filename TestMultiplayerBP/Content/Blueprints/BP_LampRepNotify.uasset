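; BP_LampRepNotify is a lamp Blueprint whose spot light alternates between red and blue, demonstrating RepNotify replication.
; From BeginPlay, only the authority changes SpotLightColor, waiting three seconds before each switch and looping through the RepeatSeq custom event.
; OnRep_SpotLightColor converts the value to a linear color and applies it to the spot light, identically on authority and remote.
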(event `self.ReceiveBeginPlay`
  ;[1 1 1] Update variable which stores light color
  (`/Engine/EditorBlueprintResources/ActorMacros.Switch Has Authority` :!label _label
    (:`Authority`
      (`KismetSystemLibrary.Delay` 3.0)
      (set `self.SpotLightColor` (`self.RedScalar`))
      (`KismetSystemLibrary.Delay` 3.0)
      (set `self.SpotLightColor` (`self.BlueScalar`))
      (`self.RepeatSeq`))))

(event `RepeatSeq`
  ;[1 1 1] Update variable which stores light color
  (goto _label))

(event `self.ReceiveTick`
  (params (DeltaSeconds :type "Float (single-precision)")))

(fn `OnRep_SpotLightColor`
  (bind _returnvalue (`KismetMathLibrary.Conv_ColorToLinearColor` (`self.SpotLightColor`)))
  (`/Engine/EditorBlueprintResources/ActorMacros.Switch Has Authority`
    (:`Authority`
      (`LightComponent.SetLightColor` (`self.SpotLight`) _returnvalue true))
    (:`Remote`
      (`LightComponent.SetLightColor` (`self.SpotLight`) _returnvalue true))))

(fn `UserConstructionScript`)