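; Example actor, apparently for a network relevancy demo, with a spotlight that switches on while something overlaps its capsule.
; Capsule begin and end overlap events check for authority, then call functions that show or hide the spotlight.
; The visibility change is not replicated, so only the server sees the light change.
; The construction script fills a text render label from a description variable.
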(event `self.Capsule.OnComponentBeginOverlap`
  (params (OverlappedComponent :type "PrimitiveComponent Object Reference") (OtherActor :type "Actor Object Reference") (OtherComp :type "PrimitiveComponent Object Reference") (OtherBodyIndex :type Integer) (bFromSweep :type Boolean) (SweepResult :type "HitResult Structure (by ref)"))
  ;[1 1 1] If server, Turn on light (only visible to server since not replicated)
  (`/Engine/EditorBlueprintResources/ActorMacros.Switch Has Authority`
    (:`Authority`
      (`self.TurnOnLight`))))

(event `self.Capsule.OnComponentEndOverlap`
  (params (OverlappedComponent :type "PrimitiveComponent Object Reference") (OtherActor :type "Actor Object Reference") (OtherComp :type "PrimitiveComponent Object Reference") (OtherBodyIndex :type Integer))
  ;[1 1 1] If server, turn off light (only visible to server)
  (`/Engine/EditorBlueprintResources/ActorMacros.Switch Has Authority`
    (:`Authority`
      (`self.TurnOffLight`))))

(fn `TurnOffLight`
  (`SceneComponent.SetVisibility` (`self.SpotLight`) false false))

(fn `TurnOnLight`
  (`SceneComponent.SetVisibility` (`self.SpotLight`) true false))

(fn `UserConstructionScript`
  (`TextRenderComponent.K2_SetText` (`self.TextRender`) (`self.Description`)))