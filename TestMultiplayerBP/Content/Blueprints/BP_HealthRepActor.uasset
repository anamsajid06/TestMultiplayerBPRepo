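; Actor that demonstrates variable replication with a health value shown on a text component.
; On the server, BeginPlay sets HealthRep to 100 and starts a looping timer that calls DecrementHealth to lower it by one every few seconds.
; Every Tick, each instance writes HealthRep into HealthTxt, so clients display whatever value reaches them.
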(event `self.ReceiveBeginPlay`
  ;[1 1 1] if server, decrement health after every 3 secs
  (`/Engine/EditorBlueprintResources/ActorMacros.Switch Has Authority`
    (:`Authority`
      (set `self.Health_Rep` 100)
      (`KismetSystemLibrary.K2_SetTimer` null "DecrementHealth" 3.0 true))))

(event `self.ReceiveTick`
  (params (DeltaSeconds :type "Float (single-precision)"))
  ;[1 1 1] Update Health Text
  (`TextRenderComponent.K2_SetText` (`self.HealthTxt`) (`KismetTextLibrary.Conv_StringToText` (`KismetStringLibrary.BuildString_Int` "" "Replicated Health: " (`self.Health_Rep`)))))

(fn `DecrementHealth`
  (set `self.Health_Rep` (- (`self.Health_Rep`) 1)))

(fn `UserConstructionScript`)